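; Base enemy death gameplay ability that plays a death montage and hands a dissolve effect to the dying enemy.
; On activation it starts the montage and fires the death sound Gameplay Cue if its tag is valid.
; The ability ends when the montage completes, blends out or is interrupted.
; On end it passes a valid dissolve Niagara system to the enemy character through OnEnemyDiedMessage.
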(event `self.K2_ActivateAbility`
  (bind _deathsoundgameplaycuetag (`self.DeathSoundGamePlayCueTag`))
  (`KismetSystemLibrary.PrintString` "Death")
  (`AbilityTask_PlayMontageAndWait.CreatePlayMontageAndWaitProxy` "None" (`self.Montage to Play_0`)
    (:`then`
      (if (`BlueprintGameplayTagLibrary.IsGameplayTagValid` _deathsoundgameplaycuetag)
        (`self.K2_ExecuteGameplayCue` _deathsoundgameplaycuetag)))
    (:`OnCompleted`
      (`self.K2_EndAbility` :!label _label))
    (:`OnBlendOut`
      (goto _label))
    (:`OnInterrupted`
      (goto _label))))

(event `self.K2_OnEndAbility`
  (params (bWasCancelled :type Boolean))
  (bind _disslove_niagara_system (`self.Disslove Niagara System`)
    (:`then`
      (message `/Game/Blueprints/Enemy/BPI_EnemyDeath.OnEnemyDied` (`self.GetEnemyCharacterFromActorInfo`) _disslove_niagara_system))
    (:`else`)))