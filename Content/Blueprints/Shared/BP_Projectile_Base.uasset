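; Base projectile Blueprint that supplies the sound and visual effects for a projectile's launch, flight and impact.
; On BeginPlay it plays an optional spawn sound, attaches a flight sound to the root and spawns a Niagara muzzle effect along its forward vector.
; The OnSpawnProjectileFX event stores the hit location, then plays the impact sound and optional effect there.
; Movement and hit detection are absent from these graphs.
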(event `self.ReceiveBeginPlay`
  (`|ExecutionSequence`
    (:`then_0`
      (bind _spawnsound (`self.SpawnSound`)
        (:`then`
          (`GameplayStatics.PlaySoundAtLocation` _spawnsound (`self.K2_GetActorLocation`) (struct) 1.0 1.0 0.0 null null null null))
        (:`else`)))
    (:`then_1`
      (bind _fliedsound (`self.FliedSound`)
        (:`then`
          (`GameplayStatics.SpawnSoundAttached` _fliedsound (`self.RootComponent`) "None" (0.0 0.0 0.0) (struct) "KeepRelativeOffset" true 1.0 1.0 0.0 null null))
        (:`else`)))
    (:`then_2`
      (bind _muzzlefx (`self.MuzzleFX`)
        (:`then`
          (`NiagaraFunctionLibrary.SpawnSystemAtLocation` _muzzlefx (`self.K2_GetActorLocation`) (`KismetMathLibrary.Conv_VectorToRotator` (`self.GetActorForwardVector`))))
        (:`else`)))))

(event `self.BP_OnSpawnProjectileFX`
  (params (HitLocation :type "Vector Structure (by ref)"))
  (set `self.Hit Location` HitLocation)
  (`|ExecutionSequence`
    (:`then_0`
      (`GameplayStatics.PlaySoundAtLocation` (`self.ImpactSoundToPlay`) (`self.Hit Location`) (struct) 1.0 1.0 0.0 null null null null))
    (:`then_1`
      (bind _impactfxtoplay (`self.ImpactFXToPlay`)
        (:`then`
          (`NiagaraFunctionLibrary.SpawnSystemAtLocation` _impactfxtoplay (`self.Hit Location`)))
        (:`else`)))))

(fn `UserConstructionScript`)