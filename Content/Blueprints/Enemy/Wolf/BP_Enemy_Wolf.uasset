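; BP_Enemy_Wolf is the wolf enemy character, extending parent behavior for BeginPlay and Tick.
; Each tick, while the wolf carries the Enemy.Wolf.Status.Alert tag, it reads the TargetActor object from its AI controller's Blackboard.
; It passes that actor's location to LookAtLocation on ABP_Enemy_Wolf, so the animation Blueprint receives a live look-at point.
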(event `self.ReceiveBeginPlay`
  (`parent.ReceiveBeginPlay`))

(event `self.ReceiveTick`
  (params (DeltaSeconds :type "Float (single-precision)"))
  (`parent.ReceiveTick` DeltaSeconds)
  (bind _asabp_enemy_wolf (cast `/Game/Blueprints/Enemy/Wolf/AnimBP/ABP_Enemy_Wolf` (`SkeletalMeshComponent.GetAnimInstance` (`self.Mesh`))))
  (`WarFunctionLibrary.BP_DoesActorHaveTag` self (struct :`TagName` "Enemy.Wolf.Status.Alert")
    (:`Yes`
      (set `/Game/Blueprints/Enemy/ABP_EnemyBase_Wolf.Look At Location` (`self.K2_GetActorLocation` (cast `Actor` (`BlackboardComponent.GetValueAsObject` (`AIController.Blackboard` (`AIBlueprintHelperLibrary.GetAIController` self)) "TargetActor") :!pure true)) _asabp_enemy_wolf))))

(fn `UserConstructionScript`
  (`parent.UserConstructionScript`))