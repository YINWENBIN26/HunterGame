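; Base AI controller for enemies that starts their behavior tree when they are possessed.
; After a short delay on possess, it runs the configured behavior tree if one is valid.
; It then seeds the blackboard with the pawn's default max walk speed from its character movement and clears the abort-all-logic flag.
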(event `self.ReceivePossess`
  (params (PossessedPawn :type "Pawn Object Reference"))
  (`KismetSystemLibrary.Delay` 0.2)
  (bind _behaviortreetorun (`self.BehaviorTreeToRun`)
    (:`then`
      (`self.RunBehaviorTree` _behaviortreetorun)
      (`BlackboardComponent.SetValueAsFloat` (`self.Blackboard`) "DefaultMaxWalkSpeed" (`CharacterMovementComponent.MaxWalkSpeed` (`Character.CharacterMovement` (cast `Character` PossessedPawn :!pure true))))
      (`BlackboardComponent.SetValueAsBool` (`self.Blackboard`) "ShouldAbortAllLogic" false))
    (:`else`)))

(fn `UserConstructionScript`)